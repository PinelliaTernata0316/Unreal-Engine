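; BP_projectile is a short-lived player projectile that destroys itself after a brief delay.
; Each tick, unless Isdead, it moves along world X at its own forward speed plus the player's ForwardSpeed.
; Its sphere overlap destroys a HealthPack or BP_Enemy along with the projectile when BPPlayer is valid, adding to the player's Score only for enemies.
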(event `self.ReceiveBeginPlay`
  (`KismetSystemLibrary.Delay` 0.7)
  (`self.K2_DestroyActor`))

(event `self.ReceiveTick`
  (params (DeltaSeconds :type "Float (single-precision)"))
  (if (not (`self.Isdead`))
    (`self.K2_AddActorWorldOffset` (`KismetMathLibrary.MakeVector` (* DeltaSeconds (+ (`self.ForwardSpeed`) (`/Game/InfiniteMatrix/Blueprints/BP_Player.ForwardSpeed` (`self.BP_Player`))))))))

(event `self.Sphere.OnComponentBeginOverlap`
  (params (OverlappedComponent :type "PrimitiveComponent Object Reference") (OtherActor :type "Actor Object Reference") (OtherComp :type "PrimitiveComponent Object Reference") (OtherBodyIndex :type Integer) (bFromSweep :type Boolean) (SweepResult :type "HitResult Structure (by ref)"))
  (bind _bp_player (`self.BP_Player`))
  (`|ExecutionSequence`
    (:`then_0`
      (bind _ashealth_pack (cast `/Game/InfiniteMatrix/Blueprints/HealthPack` OtherActor))
      (`/Engine/EditorBlueprintResources/StandardMacros.IsValid` (`self.BP_Player`)
        (:`Is Valid`
          (`self.K2_DestroyActor` _ashealth_pack)
          (`self.K2_DestroyActor`))))
    (:`then_1`
      (bind _asbp_enemy (cast `/Game/InfiniteMatrix/Blueprints/BP_Enemy` OtherActor))
      (`/Engine/EditorBlueprintResources/StandardMacros.IsValid` _bp_player
        (:`Is Valid`
          (set `/Game/InfiniteMatrix/Blueprints/BP_Player.Score` (+ (`/Game/InfiniteMatrix/Blueprints/BP_Player.Score` _bp_player) 1.0) _bp_player)
          (`self.K2_DestroyActor` _asbp_enemy)
          (`self.K2_DestroyActor`))))))

(fn `UserConstructionScript`)