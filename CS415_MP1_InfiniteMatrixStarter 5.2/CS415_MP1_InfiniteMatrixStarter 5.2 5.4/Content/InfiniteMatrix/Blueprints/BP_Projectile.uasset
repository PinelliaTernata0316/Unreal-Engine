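; BP_Projectile is a short-lived shot that flies along world X and destroys itself 0.7 seconds after spawning.
; Tick moves it with a swept world offset, at the player's ForwardSpeed plus a fixed bonus so it outpaces the player.
; A StaticMesh overlap with a BP_Enemy destroys both and increments the player's Score.
; An overlap with a BP_HealthPack destroys both without any reward.
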(event `self.ReceiveBeginPlay`
  (`KismetSystemLibrary.Delay` 0.7)
  (`self.K2_DestroyActor`))

(event `self.ReceiveTick`
  (params (DeltaSeconds :type "Float (single-precision)"))
  (`self.K2_AddActorWorldOffset` (`KismetMathLibrary.MakeVector` (* DeltaSeconds (+ (`/Game/InfiniteMatrix/Blueprints/BP_Player.ForwardSpeed` (`self.BP_player`)) 1000.0))) true))

(event `self.StaticMesh.OnComponentBeginOverlap`
  (params (OverlappedComponent :type "PrimitiveComponent Object Reference") (OtherActor :type "Actor Object Reference") (OtherComp :type "PrimitiveComponent Object Reference") (OtherBodyIndex :type Integer) (bFromSweep :type Boolean) (SweepResult :type "HitResult Structure (by ref)"))
  (bind _bp_player (`self.BP_player`))
  (`|ExecutionSequence`
    (:`then_0`
      (bind _asbp_enemy (cast `/Game/InfiniteMatrix/Blueprints/BP_Enemy` OtherActor))
      (`/Engine/EditorBlueprintResources/StandardMacros.IsValid` _bp_player
        (:`Is Valid`
          (set `/Game/InfiniteMatrix/Blueprints/BP_Player.Score` (+ (`/Game/InfiniteMatrix/Blueprints/BP_Player.Score` _bp_player) 1) _bp_player)
          (`self.K2_DestroyActor` _asbp_enemy)
          (`self.K2_DestroyActor`))))
    (:`then_1`
      (bind _asbp_health_pack (cast `/Game/InfiniteMatrix/Blueprints/BP_HealthPack` OtherActor))
      (`/Engine/EditorBlueprintResources/StandardMacros.IsValid` (`self.BP_player`)
        (:`Is Valid`
          (`self.K2_DestroyActor` _asbp_health_pack)
          (`self.K2_DestroyActor`))))))

(fn `UserConstructionScript`)